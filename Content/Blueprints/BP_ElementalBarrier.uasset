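; BP_ElementalBarrier is an elemental barrier that ends the game when a third-person character without the matching immunity enters it.
; On BeginPlay it prints its ElementalType and labels its text render as Fire, Ice, Earth or Wind, mapped from Melee, Projectile, Explosion and Environment values.
; Overlapping the cube compares that type to the character's ElementalImmunity; a mismatch prints a death message, then quits the game after a short delay.
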(event OnComponentBeginOverlap(Cube)
  (params (OverlappedComponent :type Primitive%20Component%20Object%20Reference) (OtherActor :type Actor%20Object%20Reference) (OtherComp :type Primitive%20Component%20Object%20Reference) (OtherBodyIndex :type Integer) (bFromSweep :type Boolean) (SweepResult :type Hit%20Result%20Structure%20%28by%20ref%29))
  (bind _asbp_third_person_character (Utilities|Casting|CastToBP_ThirdPersonCharacter OtherActor))
  (if (not (Utilities|Enum|Equal(Enum) (Variables|Default|GetElemental%20Type) (Variables|/Game/ThirdPerson/Blueprints/BP_ThirdPersonCharacter.BP_ThirdPersonCharacter_C|GetElemental%20Immunity _asbp_third_person_character)))
    (Development|PrintString "You're Dead!")
    (Utilities|FlowControl|Delay 2.0)
    (Game|QuitGame 0 "Quit" false)))

(event EventBeginPlay
  (bind _elemental_type (Variables|Default|GetElemental%20Type))
  (Development|PrintString (Utilities|String|ToString(Text) (|GenerictoText _elemental_type)))
  (switch Utilities|FlowControl|Switch|SwitchonE_DamageType _elemental_type
    (:NewEnumerator1
      (Rendering|Components|TextRender|SetText (Variables|Default|GetTextRender) (Utilities|Text|MakeLiteralText "Barrier of Fire")))
    (:NewEnumerator2
      (Rendering|Components|TextRender|SetText (Variables|Default|GetTextRender) (Utilities|Text|MakeLiteralText "Barrier of Ice")))
    (:NewEnumerator3
      (Rendering|Components|TextRender|SetText (Variables|Default|GetTextRender) (Utilities|Text|MakeLiteralText "Barrier of Earth")))
    (:NewEnumerator4
      (Rendering|Components|TextRender|SetText (Variables|Default|GetTextRender) (Utilities|Text|MakeLiteralText "Barrier of Wind")))))

(fn ConstructionScript)
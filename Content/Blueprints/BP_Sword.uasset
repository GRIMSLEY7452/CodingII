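; Sword item that a character can pick up, use and drop.
; PickUp snaps it to the given skeletal mesh's right-hand socket and disables collision on the sword mesh.
; Primary and secondary use only print placeholder text.
; Drop detaches it in world space, restores collision and simulates physics briefly, then switches physics off after a delay.
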(event EventBeginPlay)

(event EventDrop
  (Transformation|DetachFromActor "KeepWorld" "KeepWorld" "KeepRelative")
  (Physics|SetSimulatePhysics (Variables|Default|GetSM_uitlbiaga_tier_2) true)
  (Collision|SetCollisionEnabled (Variables|Default|GetSM_uitlbiaga_tier_2) "QueryAndPhysics")
  (Utilities|FlowControl|Delay 2.0)
  (Physics|SetSimulatePhysics (Variables|Default|GetSM_uitlbiaga_tier_2) false))

(event EventUsePrimary
  (Development|PrintText "Swish!"))

(event EventPickUp
  (params (SkeletalMesh :type Skeletal%20Mesh%20Component%20Object%20Reference))
  (Development|PrintText (Utilities|Text|FormatText "{name} is getting picked up and attached to {mesh}." (Utilities|String|MakeLiteralString "Sword") SkeletalMesh) true true "(R=1.000000,G=0.000000,B=0.806917,A=1.000000)")
  (Transformation|AttachComponentToComponent SkeletalMesh "hand_r" "SnapToTarget" "SnapToTarget" "KeepRelative" true)
  (Collision|SetCollisionEnabled (Variables|Default|GetSM_uitlbiaga_tier_2) "NoCollision"))

(event EventUseSecondary
  (Development|PrintText "Slash!"))

(fn ConstructionScript)
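; Grenade pickup actor that increments the player's grenade count when the third-person character overlaps its sphere.
; On pickup it registers itself in the save game mode's collected-grenade level state, prints the new count, plays a sound and destroys itself.
; An AlreadyCollected event, meant to be called by GM_Save_Load, destroys grenades that were collected earlier.
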(event OnComponentBeginOverlap(Sphere)
  (params (OverlappedComponent :type Primitive%20Component%20Object%20Reference) (OtherActor :type Actor%20Object%20Reference) (OtherComp :type Primitive%20Component%20Object%20Reference) (OtherBodyIndex :type Integer) (bFromSweep :type Boolean) (SweepResult :type Hit%20Result%20Structure%20%28by%20ref%29))
  (bind _asbp_third_person_character (Utilities|Casting|CastToBP_ThirdPersonCharacter OtherActor))
  (bind _asgm_save_load (Utilities|Casting|CastToGM_Save_Load (Game|GetGameMode)))
  (Utilities|Array|AddUnique (Variables|/Game/Blueprints/Saving_and_Loading/SG_LevelState.SG_LevelState_C|GetCollectedGrenades (Variables|/Game/Blueprints/Saving_and_Loading/GM_Save_Load.GM_Save_Load_C|GetSG_LevelState _asgm_save_load)) self)
  (Variables|/Game/ThirdPerson/Blueprints/BP_ThirdPersonCharacter.BP_ThirdPersonCharacter_C|SetGrenade%20Count _asbp_third_person_character (+ (Variables|/Game/ThirdPerson/Blueprints/BP_ThirdPersonCharacter.BP_ThirdPersonCharacter_C|GetGrenade%20Count _asbp_third_person_character) 1))
  (Development|PrintString (Utilities|String|Append "The Player has " (Utilities|String|ToString(Integer) (Variables|/Game/ThirdPerson/Blueprints/BP_ThirdPersonCharacter.BP_ThirdPersonCharacter_C|GetGrenade%20Count _asbp_third_person_character)) " grenade(s)."))
  (Audio|PlaySoundatLocation "/Game/Audio/Pickup_Key_Real.Pickup_Key_Real" (Transformation|GetWorldLocation (Variables|Default|GetDefaultSceneRoot)) "0, 0, 0" 1.0 1.0 0.0 0 0 0 0)
  (Actor|DestroyActor) ; Destroy this key
)

(event Custom|Already%20Collected
  ;[0.15 0.15 0.15 0.5] If the grenade has already been collected,  destroy it. GM_Save_Load will call this function.
  (Actor|DestroyActor))

(fn ConstructionScript)
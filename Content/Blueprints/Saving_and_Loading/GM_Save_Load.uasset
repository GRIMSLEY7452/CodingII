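; Game mode that owns saving and loading of player stats and per-level state, loading both on BeginPlay.
; Player stats use a fixed slot and restore Stamina, Health and Mana to the third-person character.
; Level state uses a slot named after the level, replaying collected coins and opened doors.
; Missing saves get fresh save objects; save events write the held objects to disk without gathering values.
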(event Custom|LoadPlayerStats
  (bind _returnvalue (SaveGame|DoesSaveGameExist "PlayerSave"))
  (if _returnvalue
    (bind _returnvalue_2 (SaveGame|LoadGamefromSlot "PlayerSave"))
    (bind _assg_player_stats (Utilities|Casting|CastToSG_Player_Stats _returnvalue_2))
    (Variables|Default|SetSG_Player_Stats _assg_player_stats)
    (bind _asbp_third_person_character (Utilities|Casting|CastToBP_ThirdPersonCharacter (Game|GetPlayerCharacter 0)))
    (Variables|/Game/ThirdPerson/Blueprints/BP_ThirdPersonCharacter.BP_ThirdPersonCharacter_C|SetStamina _asbp_third_person_character (Variables|/Game/Blueprints/Saving_and_Loading/SG_Player_Stats.SG_Player_Stats_C|GetStamina (Variables|Default|GetSG_Player_Stats))) ; The player's stamina.
    (Variables|/Game/ThirdPerson/Blueprints/BP_ThirdPersonCharacter.BP_ThirdPersonCharacter_C|SetHealth _asbp_third_person_character (Variables|/Game/Blueprints/Saving_and_Loading/SG_Player_Stats.SG_Player_Stats_C|GetHealth (Variables|Default|GetSG_Player_Stats)))
    (Variables|/Game/ThirdPerson/Blueprints/BP_ThirdPersonCharacter.BP_ThirdPersonCharacter_C|SetMana _asbp_third_person_character (Variables|/Game/Blueprints/Saving_and_Loading/SG_Player_Stats.SG_Player_Stats_C|GetMana (Variables|Default|GetSG_Player_Stats)))
    (Development|PrintText "PlayerStats have been loaded." true true "(R=1.000000,G=0.071304,B=0.000000,A=1.000000)" 8.0)
    (else
      (bind _returnvalue_3 (SaveGame|CreateSaveGameObject "/Game/Blueprints/Saving_and_Loading/SG_Player_Stats.SG_Player_Stats_C"))
      (Variables|Default|SetSG_Player_Stats _returnvalue_3))))

(event Custom|Save%20Player%20Stats
  (bind _returnvalue (SaveGame|SaveGametoSlot (Variables|Default|GetSG_Player_Stats) "PlayerSave"))
  (if _returnvalue
    (Development|PrintText "Player Stats Written to Save Game File." true true "(R=0.086649,G=1.000000,B=0.007653,A=1.000000)" 8.0)
    (else
      (Development|PrintText "Player Stats Could Not be Written to Save Game File." true true "(R=1.000000,G=0.000000,B=0.000000,A=1.000000)" 8.0))))

(event Custom|Save%20Level%20State
  (bind _returnvalue (Game|GetCurrentLevelName true))
  (SaveGame|SaveGametoSlot (Variables|Default|GetSG_LevelState) _returnvalue)
  (if true
    (Development|PrintText "Level State Written to Save Game File.")
    (else
      (Development|PrintText "Player Stats Could Not Be Written to Save Game File."))))

(event Custom|Load%20Level%20State
  (bind _returnvalue (Game|GetCurrentLevelName true))
  (bind _returnvalue_2 (SaveGame|DoesSaveGameExist _returnvalue))
  (if _returnvalue_2
    (bind _returnvalue_3 (SaveGame|LoadGamefromSlot _returnvalue))
    (bind _assg_level_state (Utilities|Casting|CastToSG_LevelState _returnvalue_3))
    (bind _output_get (Variables|Default|SetSG_LevelState _assg_level_state))
    (for _array_element (Variables|/Game/Blueprints/Saving_and_Loading/SG_LevelState.SG_LevelState_C|GetCollectedCoins _output_get)
      (Utilities|IsValid _array_element ; What if the coin isn't in the level?
        (:Is%20Valid
          (Default|AlreadyCollected _array_element))))
    (Development|PrintText "Coin State Loaded.")
    (for _array_element_2 (Variables|/Game/Blueprints/Saving_and_Loading/SG_LevelState.SG_LevelState_C|GetOpenDoors _output_get)
      (Default|OpenDoorAgain _array_element_2))
    (Development|PrintString "Opened Doors Loaded.")
    (else
      (bind _returnvalue_4 (SaveGame|CreateSaveGameObject "/Game/Blueprints/Saving_and_Loading/SG_LevelState.SG_LevelState_C"))
      (Variables|Default|SetSG_LevelState _returnvalue_4))))

(event EventBeginPlay
  (Development|PrintText "Loading the Save_Load Game Mode." true true "(R=1.000000,G=0.333785,B=0.000000,A=1.000000)")
  (CallFunction|LoadPlayerStats)
  (CallFunction|LoadLevelState))

(fn ConstructionScript)
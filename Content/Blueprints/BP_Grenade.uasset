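; BP_Grenade is a timed grenade that destroys nearby turrets when it explodes.
; Three seconds after BeginPlay it spawns explosion particles and sound at the grenade body, then hides itself.
; It destroys every BP_Turret overlapping its sphere and adds an entry to the level state's Turrets list in GM_Save_Load.
; The hidden grenade destroys itself after a further short delay.
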(event EventBeginPlay
  (Utilities|FlowControl|Delay 3.0)
  (Effects|SpawnEmitteratLocation "/Game/StarterContent/Particles/P_Explosion.P_Explosion" (Transformation|GetWorldLocation (Variables|Default|GetGrenade_high_Body1)))
  (Audio|PlaySoundatLocation "/Game/Audio/Explosion.Explosion" (Transformation|GetWorldLocation (Variables|Default|GetGrenade_high_Body1)) "0, 0, 0" 1.0 1.0 0.0 0 0 0 0)
  (Rendering|SetActorHiddenInGame true)
  (Utilities|FlowControl|Sequence
    (:then_0
      (bind _output_get (Variables|Default|SetOverlapping%20Actors (Collision|GetOverlappingActors (Variables|Default|GetSphere) "/Game/Blueprints/BP_Turret.BP_Turret_C" :!class /Script/Engine.PrimitiveComponent)))
      (for _array_element _output_get
        (bind _asbp_turret (Utilities|Casting|CastToBP_Turret _array_element))
        (Actor|DestroyActor _asbp_turret)
        (bind _asgm_save_load (Utilities|Casting|CastToGM_Save_Load (Game|GetGameMode)))
        (Utilities|Array|AddUnique (Variables|/Game/Blueprints/Saving_and_Loading/SG_LevelState.SG_LevelState_C|GetTurrets (Variables|/Game/Blueprints/Saving_and_Loading/GM_Save_Load.GM_Save_Load_C|GetSG_LevelState _asgm_save_load)) 0)))
    (:then_1
      (Utilities|FlowControl|Delay 2.0)
      (Actor|DestroyActor))))

(fn ConstructionScript)
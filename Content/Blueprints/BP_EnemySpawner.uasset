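; BP_EnemySpawner populates the level with randomized AI enemies when play begins.
; On BeginPlay it finds every BP_EnemySpawnPoint and, with a 50% chance per point, spawns a BP_AiMoveTo at that transform.
; Each spawned AI gets a random name on its text component, a random skeletal mesh and random materials in its first two slots, all drawn from hardcoded arrays.
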(event EventBeginPlay
  (Development|PrintString "Enemy spawner is active.")
  (bind _outactors (Actor|GetAllActorsOfClass "/Game/Blueprints/BP_EnemySpawnPoint.BP_EnemySpawnPoint_C"))
  (for _array_element _outactors
    (if (Math|Random|RandomBoolwithWeight 0.5)
      (bind _returnvalue (Game|SpawnActorfromClass "/Game/AI_Blueprints/BP_AiMoveTo.BP_AiMoveTo_C" (Transformation|GetActorTransform _array_element) "Undefined" "MultiplyWithRoot" 0 0))
      (Rendering|Components|TextRender|SetText (Variables|/Game/AI_Blueprints/BP_AiMoveTo.BP_AiMoveTo_C|GetAI%20Name%20Text _returnvalue) (Utilities|Text|MakeLiteralText (.OutItem (Utilities|Array|Random (Utilities|Array|MakeArray "Matthew" "Mark" "Luke" "John" "Daniel" "Job" "Moses" "Solomon")))))
      (Components|SkeletalMesh|SetSkeletalMeshAsset (Variables|/Script/Engine.Character|GetMesh _returnvalue) (.OutItem (Utilities|Array|Random (Utilities|Array|MakeArray "/Game/SCK_Casual01/Models/Premade_Characters/MESH_PC_00.MESH_PC_00" "/Game/PolygonStarter/EpicContent/Mannequin/Character/Mesh/SK_Mannequin.SK_Mannequin" "/Game/PolygonStarter/Models/Vehicles/SK_PolygonCity_Veh_Car_Small_01.SK_PolygonCity_Veh_Car_Small_01" "/Game/PolygonStarter/Models/Vehicles/SK_Veh_Plane_Stunt_01.SK_Veh_Plane_Stunt_01" "/Game/SCK_Casual01/Models/MESH_A_04.MESH_A_04" "/Game/SCK_Casual01/Models/MESH_L_01.MESH_L_01" "/Game/SCK_Casual01/Models/MESH_T_01.MESH_T_01" "/Game/PolygonStarter/Models/Characters/SK_Chr_Female_Face_01.SK_Chr_Female_Face_01"))))
      (Rendering|Material|SetMaterial (Variables|/Script/Engine.Character|GetMesh _returnvalue) 0 (.OutItem (Utilities|Array|Random (Utilities|Array|MakeArray "/Engine/EditorMeshes/ColorCalibrator/M_ChromeBall.M_ChromeBall" "/Engine/EditorMeshes/ColorCalibrator/M_ClearCoat.M_ClearCoat" "/Niagara/DefaultAssets/GeometryCache/M_DefaultGeometryCacheMaterial_Red.M_DefaultGeometryCacheMaterial_Red" "/Game/Characters/Mannequins/Materials/M_Mannequin.M_Mannequin" "/Game/PolygonStarter/Materials/M_Simple_Sky_01.M_Simple_Sky_01" "/Game/SCK_Casual01/Materials/Master_Materials/MAT_H_A1.MAT_H_A1" "/Engine/EngineDebugMaterials/MAT_LevelColorationLitLightmapUV.MAT_LevelColorationLitLightmapUV" "/Game/SCK_Casual01/Materials/Master_Materials/MAT_T_01.MAT_T_01"))))
      (Rendering|Material|SetMaterial (Variables|/Script/Engine.Character|GetMesh _returnvalue) 1 (.OutItem (Utilities|Array|Random (Utilities|Array|MakeArray "/Niagara/DefaultAssets/GeometryCache/M_DefaultGeometryCacheMaterial_Blue.M_DefaultGeometryCacheMaterial_Blue" "/Niagara/DefaultAssets/GeometryCache/M_DefaultGeometryCacheMaterial_Green.M_DefaultGeometryCacheMaterial_Green" "/DatasmithContent/Materials/CE_OpaqueReference.CE_OpaqueReference" "/Game/Fab/Door/door_glb/Materials/Door_001.Door_001" "/Game/SCK_Casual01/Materials/Master_Materials/MAT_L_01.MAT_L_01" "/Game/SCK_Casual01/Materials/Material_Instances/Mi_A_01_4.Mi_A_01_4" "/Game/Materials/MI_FlatRed.MI_FlatRed" "/Game/SCK_Casual01/Materials/Master_Materials/MAT_T_00.MAT_T_00")))))))

(fn ConstructionScript)
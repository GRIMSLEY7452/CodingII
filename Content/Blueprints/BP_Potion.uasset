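; BP_Potion is a holdable potion item with pick up, primary use, secondary use and drop events.
; Pick up snaps it to the hand_r socket of the given skeletal mesh and disables the bottle's collision.
; Drop detaches it, restores collision and simulates physics on the bottle for a short delay before switching physics off.
; Both use events are placeholders that only print drink or throw messages.
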(event EventBeginPlay)

(event EventPickUp
  (params (SkeletalMesh :type Skeletal%20Mesh%20Component%20Object%20Reference))
  (Development|PrintText (Utilities|Text|FormatText "{name} is getting picked up and attached to {mesh}." (Utilities|String|MakeLiteralString "Potion") SkeletalMesh) true true "(R=1.000000,G=0.000000,B=0.806917,A=1.000000)")
  (Transformation|AttachComponentToComponent SkeletalMesh "hand_r" "SnapToTarget" "SnapToTarget" "KeepRelative" true)
  (Collision|SetCollisionEnabled (Variables|Default|GetPotion%20Bottle) "NoCollision"))

(event EventUsePrimary
  (Development|PrintText "Glug glug glug."))

(event EventUseSecondary
  (Development|PrintText "Crash!!! (You threw the potion)"))

(event EventDrop
  (Transformation|DetachFromActor "KeepWorld" "KeepWorld" "KeepRelative")
  (Physics|SetSimulatePhysics (Variables|Default|GetPotion%20Bottle) true)
  (Collision|SetCollisionEnabled (Variables|Default|GetPotion%20Bottle) "QueryAndPhysics")
  (Utilities|FlowControl|Delay 2.0)
  (Physics|SetSimulatePhysics (Variables|Default|GetPotion%20Bottle) false))

(fn ConstructionScript)
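; Base enemy character Blueprint with patrol, aggro, melee attack and death, exposing helpers that AI behavior tasks can use.
; Attack plays a kick montage, applies damage to player characters inside a debug-drawn sphere overlap, and signals when finished.
; Aggro swaps the mesh to a red material, while patrol steps along an assigned spline route, reversing at either end.
; Point damage reduces health and triggers a ragdoll with radial force at zero.
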(event Custom|Attack
  (bind _attacksphere (Variables|Default|GetAttackSphere))
  (bind _attackrange (Variables|Default|GetAttackRange))
  (bind _returnvalue (Transformation|GetWorldLocation _attacksphere))
  (Development|PrintString "Attacking Player!")
  (Animation|Montage|PlayMontage (Variables|Character|GetMesh) "/Game/CloseCombatAnimSet/Animations/InPlace/Attacks/NinjaWheelKick_Montage.NinjaWheelKick_Montage"
    (:then
      (bind _outactors (Collision|SphereOverlapActors _returnvalue _attackrange (Utilities|Array|MakeArray "ObjectTypeQuery3") "/Game/ThirdPerson/Blueprints/BP_ThirdPersonCharacter.BP_ThirdPersonCharacter_C" (Utilities|Array|MakeArray self)))
      (Rendering|Debug|DrawDebugSphere _returnvalue _attackrange 12 "(R=1.000000,G=0.025531,B=0.000000,A=1.000000)" 2.0)
      (for _array_element _outactors
        (Game|Damage|ApplyDamage _array_element 0.2 (Pawn|GetController) self "/Script/Engine.DamageType")))
    (:OnCompleted
      (Default|CallAttackFinished :!label _label))
    (:OnInterrupted
      (goto _label))))

(event Custom|Get%20Aggro
  (Rendering|Material|SetMaterial (Variables|Character|GetMesh) 0 "/Game/Materials/MI_FlatRed.MI_FlatRed")
  (Variables|Default|SetAggroed true))

(event Custom|Lose%20Aggro
  (Rendering|Material|SetMaterial (Variables|Character|GetMesh) 0 (Variables|Default|GetOriginal%20Material))
  (Variables|Default|SetAggroed false))

(event Custom|Set%20Walk%20Speed
  (params (New%20Speed :type Float%20%28double-precision%29))
  (Variables|/Script/Engine.CharacterMovementComponent|SetMaxWalkSpeed (Variables|Character|GetCharacterMovement) New%20Speed))

(event Custom|Any%20Damage
  (params (Damage :type Float%20%28double-precision%29) (Damage%20Type :type Damage%20Type%20Object%20Reference) (Instigated%20By :type Controller%20Object%20Reference) (Damage%20Causer :type Actor%20Object%20Reference)))

(event Custom|Ragdoll
  (params (Origin :type Vector))
  (bind _mesh (Variables|Character|GetMesh))
  (Physics|SetSimulatePhysics _mesh true)
  (Physics|AddRadialForce _mesh (+ Origin "0.000000,0.000000,-100.000000") 5e+02 2.5e+04 "RIF_Constant" true)
  (Pawn|Components|CharacterMovement|DisableMovement (Variables|Character|GetCharacterMovement)))

(event EventBeginPlay
  (Variables|Default|SetOriginal%20Material (Rendering|Material|GetMaterial (Variables|Character|GetMesh) 0)))

(event Game|Damage|EventPointDamage
  (params (Damage :type Float%20%28single-precision%29) (DamageType :type Damage%20Type%20Object%20Reference) (HitLocation :type Vector :default "0, 0, 0") (HitNormal :type Vector :default "0, 0, 0") (HitComponent :type Primitive%20Component%20Object%20Reference) (BoneName :type Name :default "None") (ShotFromDirection :type Vector :default "0, 0, 0") (InstigatedBy :type Controller%20Object%20Reference) (DamageCauser :type Actor%20Object%20Reference) (HitInfo :type Hit%20Result%20Structure%20%28by%20ref%29))
  (Development|PrintText (Utilities|Text|FormatText "{instigator} damaged us for {damage} damage!" InstigatedBy Damage))
  (bind _output_get (Variables|Default|SetHealth (- (Variables|Default|GetHealth) Damage)))
  (if (<= _output_get 0.0) ; Are we dead?
    (Development|PrintString "We are dead!")
    (CallFunction|Ragdoll HitLocation)))

(fn ConstructionScript)

(fn GetNextPatrolPointLocation
  (Utilities|IsValid (Variables|PatrolRoute|GetPatrol%20Route)
    (:Is%20Valid
      (Variables|PatrolRoute|SetPatrol%20Point%20Index (+ (Variables|PatrolRoute|GetPatrol%20Point%20Index) (Variables|PatrolRoute|GetPatrol%20Route%20Direction)))
      (if (or (>= (Variables|PatrolRoute|GetPatrol%20Point%20Index) (- (Spline|GetNumberOfSplinePoints (Variables|/Game/AI_Blueprints/BP_PatrolRoute.BP_PatrolRoute_C|GetRoute (Variables|PatrolRoute|GetPatrol%20Route))) 1)) (<= (Variables|PatrolRoute|GetPatrol%20Point%20Index) 0))
        (Variables|PatrolRoute|SetPatrol%20Route%20Direction (* (Variables|PatrolRoute|GetPatrol%20Route%20Direction) -1)))
      (return (Spline|GetLocationatSplinePoint (Variables|/Game/AI_Blueprints/BP_PatrolRoute.BP_PatrolRoute_C|GetRoute (Variables|PatrolRoute|GetPatrol%20Route)) (Variables|PatrolRoute|GetPatrol%20Point%20Index) "World")))
    (:Is%20Not%20Valid
      (Development|PrintString "No Patrol Route Assigned."))))

(fn GetIdealRange
  (return (Variables|Default|GetAttack%20Radius) (Variables|Default|GetStrafe%20Radius)))